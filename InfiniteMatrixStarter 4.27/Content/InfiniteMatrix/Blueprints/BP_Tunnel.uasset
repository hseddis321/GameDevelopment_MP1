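; BP_Tunnel is a tunnel segment for an endless runner, with a rotating holed wall that damages the player and destroys bullets.
; Its trigger zone asks TunnelSpawner for the next segment and, unless the wall was hit, adds score and destroys itself with its pickup and enemy.
; Wall hits can kill the player and show restart.
; Randomize functions, not called here, vary wall mesh and roll and maybe spawn a health pack or enemy.
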(event `self.ReceiveTick`
  (params (DeltaSeconds :type "Float (single-precision)"))
  (`SceneComponent.K2_AddLocalRotation` (`self.WallMesh`) (`KismetMathLibrary.MakeRotator` (* DeltaSeconds (`self.RotateSpeed`))) false false))

(event `self.TriggerZone.OnComponentBeginOverlap`
  (params (OverlappedComponent :type "PrimitiveComponent Object Reference") (OtherActor :type "Actor Object Reference") (OtherComp :type "PrimitiveComponent Object Reference") (OtherBodyIndex :type Integer) (bFromSweep :type Boolean) (SweepResult :type "HitResult Structure (by ref)"))
  (bind _asbp_player (cast `/Game/InfiniteMatrix/Blueprints/BP_Player` OtherActor))
  (`/Game/InfiniteMatrix/Blueprints/BP_TunnelSpawner.Spawn Tunnel at Spawn Point` (`self.Tunnel Spawner`))
  (if (not (`self.Hit Wall`))
    (`/Engine/EditorBlueprintResources/StandardMacros.IncrementInt` (`/Game/InfiniteMatrix/Blueprints/BP_Player.Score` _asbp_player)
      (:`  `
        (if (`self.HasHealthPack`)
          (`self.K2_DestroyActor` (`self.HealthPack`)))
        (if (`self.HasEnemy`)
          (`self.K2_DestroyActor` (`self.Enemy`)))
        (`self.K2_DestroyActor`)))))

(event `self.WallMesh.OnComponentBeginOverlap`
  (params (OverlappedComponent :type "PrimitiveComponent Object Reference") (OtherActor :type "Actor Object Reference") (OtherComp :type "PrimitiveComponent Object Reference") (OtherBodyIndex :type Integer) (bFromSweep :type Boolean) (SweepResult :type "HitResult Structure (by ref)"))
  (bind _asbp_player (cast `/Game/InfiniteMatrix/Blueprints/BP_Player` OtherActor)
    (:`then`
      (bind _output_get (set `/Game/InfiniteMatrix/Blueprints/BP_Player.Health` (- (`/Game/InfiniteMatrix/Blueprints/BP_Player.Health` _asbp_player) 25.0) _asbp_player))
      (set `self.Hit Wall` true)
      (if (<= _output_get 0.0)
        (set `/Game/InfiniteMatrix/Blueprints/BP_Player.IsDead` true _asbp_player)
        (`/Game/InfiniteMatrix/Blueprints/BP_Player.Display Restart` _asbp_player)))
    (:`CastFailed`
      (bind _asbullet (cast `/Game/InfiniteMatrix/Blueprints/Bullet` OtherActor))
      (`self.K2_DestroyActor` _asbullet))))

(fn `RandomizeEnemy`
  (if (< (`KismetMathLibrary.RandomFloatInRange` 0.0 1.0) 0.66)
    (set `self.HasEnemy` true)
    (bind _returnvalue (`|SpawnActorFromClass` "/Game/InfiniteMatrix/Blueprints/Enemy.Enemy_C" (`KismetMathLibrary.MakeTransform` (- (`SceneComponent.K2_GetComponentLocation` (`self.SpawnPoint`)) (`KismetMathLibrary.MakeVector` (`KismetMathLibrary.RandomFloatInRange` 500.0 1500.0) (`KismetMathLibrary.RandomFloatInRange` -250.0 250.0) (`KismetMathLibrary.RandomFloatInRange` -250.0 250.0)))) "Undefined" "OverrideRootScale" null null))
    (bind _output_get (set `self.Enemy` _returnvalue))
    (set `/Game/InfiniteMatrix/Blueprints/Enemy.Vertical` (< (`KismetMathLibrary.RandomFloatInRange` 0.0 1.0) 0.5) _output_get)))

(fn `RandomizeHealthPack`
  (if (< (`KismetMathLibrary.RandomFloatInRange` 0.0 1.0) 0.5)
    (set `self.HasHealthPack` true)
    (bind _returnvalue (`|SpawnActorFromClass` "/Game/InfiniteMatrix/Blueprints/Health_Pack.Health_Pack_C" (`KismetMathLibrary.MakeTransform` (- (`SceneComponent.K2_GetComponentLocation` (`self.SpawnPoint`)) (`KismetMathLibrary.MakeVector` (`KismetMathLibrary.RandomFloatInRange` 500.0 1500.0) (`KismetMathLibrary.RandomFloatInRange` -250.0 250.0) (`KismetMathLibrary.RandomFloatInRange` -250.0 250.0)))) "Undefined" "OverrideRootScale" null null))
    (set `self.HealthPack` _returnvalue)))

(fn `RandomizeWall`
  (`StaticMeshComponent.SetStaticMesh` (`self.WallMesh`) (select `int` (`KismetMathLibrary.RandomIntegerInRange` 0 3) :`0` "/Game/InfiniteMatrix/Meshes/SM_Hole_01.SM_Hole_01" :`1` "/Game/InfiniteMatrix/Meshes/SM_Hole_02.SM_Hole_02" :`2` "/Game/InfiniteMatrix/Meshes/SM_Hole_03.SM_Hole_03" :`3` "/Game/InfiniteMatrix/Meshes/SM_Hole_04.SM_Hole_04" :!type "StaticMesh Object Reference"))
  (`SceneComponent.K2_AddLocalRotation` (`self.WallMesh`) (`KismetMathLibrary.MakeRotator` (`KismetMathLibrary.RandomFloatInRange` 0.0 360.0)) false false))

(fn `UserConstructionScript`)