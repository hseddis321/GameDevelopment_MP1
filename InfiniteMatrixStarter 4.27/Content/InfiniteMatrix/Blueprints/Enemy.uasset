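; Enemy actor that patrols back and forth as a moving hazard, damaging the player and dying to bullets.
; Tick sweeps it along world Y when Vertical is set, otherwise Z, reversing at fixed world-position bounds.
; Player overlap reduces health, triggering death and the restart display at zero.
; Bullet overlap destroys the bullet, then searches all BP_Tunnel actors for this enemy's owner to destroy it and clear HasEnemy.
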(event `self.ReceiveActorBeginOverlap`
  (params (OtherActor :type "Actor Object Reference"))
  (bind _asbp_player (cast `/Game/InfiniteMatrix/Blueprints/BP_Player` OtherActor)
    (:`then`
      (bind _output_get (set `/Game/InfiniteMatrix/Blueprints/BP_Player.Health` (`KismetMathLibrary.FMax` (- (`/Game/InfiniteMatrix/Blueprints/BP_Player.Health` _asbp_player) 10.0)) _asbp_player))
      (if (<= _output_get 0.0)
        (set `/Game/InfiniteMatrix/Blueprints/BP_Player.IsDead` true _asbp_player)
        (`/Game/InfiniteMatrix/Blueprints/BP_Player.Display Restart` _asbp_player)))
    (:`CastFailed`
      (bind _asbullet (cast `/Game/InfiniteMatrix/Blueprints/Bullet` OtherActor))
      (`self.K2_DestroyActor` _asbullet)
      (bind _outactors (`GameplayStatics.GetAllActorsOfClass` "/Game/InfiniteMatrix/Blueprints/BP_Tunnel.BP_Tunnel_C"))
      (for _array_element _outactors
        (bind _enemy (`/Game/InfiniteMatrix/Blueprints/BP_Tunnel.Enemy` _array_element))
        (if (== _enemy self)
          (`self.K2_DestroyActor` _enemy)
          (set `/Game/InfiniteMatrix/Blueprints/BP_Tunnel.HasEnemy` false _array_element))))))

(event `self.ReceiveTick`
  (params (DeltaSeconds :type "Float (single-precision)"))
  (bind _is_forward (`self.is_forward`))
  (bind _speed (`self.speed`))
  (bind (_returnvalue_x _returnvalue_y _returnvalue_z) (`KismetMathLibrary.BreakVector` (`SceneComponent.K2_GetComponentLocation` (`self.DefaultSceneRoot`))))
  (if (`self.Vertical`)
    (if _is_forward
      (`self.K2_AddActorWorldOffset` (`KismetMathLibrary.MakeVector` 0.0 (* _speed DeltaSeconds)) true)
      (if (or (> _returnvalue_y 249.0) (> _returnvalue_z 249.0)) :!label _label
        (set `self.is_forward` false))
      (else
        (`self.K2_AddActorWorldOffset` (`KismetMathLibrary.MakeVector` 0.0 (* DeltaSeconds _speed -1.0)) true)
        (if (or (< _returnvalue_y -249.0) (< _returnvalue_z -249.0)) :!label _label_2
          (set `self.is_forward` true))))
    (elif _is_forward
      (`self.K2_AddActorWorldOffset` (`KismetMathLibrary.MakeVector` 0.0 0.0 (* DeltaSeconds _speed)) true)
      (goto _label)
      (else
        (`self.K2_AddActorWorldOffset` (`KismetMathLibrary.MakeVector` 0.0 0.0 (* DeltaSeconds _speed -1.0)) true)
        (goto _label_2)))))

(fn `UserConstructionScript`)